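; Lobby player controller that creates the lobby widget for the local player on possess and relays lobby state to it.
; Events forward ready-player counts, countdown updates and the set-name prompt to the widget, retrying every 0.2 seconds until it is valid.
; Showing the name prompt also disables pawn input and shows the mouse cursor through a shared input toggle.
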(event Custom|ShowSetName
  (bind _actualwidget (Variables|Default|GetactualWidget))
  ;[0 0 0] Show Set name widget
  (Utilities|IsValid _actualwidget :!label _label
    (:Is%20Valid
      (Default|ShowSetName _actualwidget)
      (CallFunction|SetEnableInput true true))
    (:Is%20Not%20Valid
      (Utilities|FlowControl|Delay 0.2)
      (goto _label))))

(event Custom|SetEnableInput
  (params (disable :type Boolean) (showMouse :type Boolean))
  (bind _self self)
  (bind _self_2 self)
  (bind _returnvalue (Pawn|GetControlledPawn _self))
  ;[0 0 0] Enable input
  (Variables|Default|SetbShowMouseCursor showMouse)
  (Utilities|IsValid _returnvalue
    (:Is%20Valid
      (if disable
        (Input|DisableInput _returnvalue _self_2)
        (else
          (Input|EnableInput _returnvalue _self_2))))))

(event Custom|UpdateCoundTown
  (params (count :type Integer))
  (bind _actualwidget (Variables|Default|GetactualWidget))
  (Utilities|IsValid _actualwidget :!label _label
    (:Is%20Valid
      (Default|UpdateCountDown _actualwidget count))
    (:Is%20Not%20Valid
      (Utilities|FlowControl|Delay 0.2)
      (goto _label))))

(event Custom|ShowReadyPlayer
  (params (players :type Integer) (totalPlayers :type Integer))
  (Utilities|IsValid (Variables|Default|GetactualWidget) :!label _label
    (:Is%20Valid
      (Default|ShowPlayersReady (Variables|Default|GetactualWidget) players totalPlayers))
    (:Is%20Not%20Valid
      (Utilities|FlowControl|Delay 0.2)
      (goto _label))))

(event Custom|EventPossess
  ;[0 0 0] Display widget lobby
  (if (Pawn|IsLocalPlayerController)
    (bind _returnvalue (UserInterface|CreateWidget "/Game/UI/Lobby/WBP_Lobby.WBP_Lobby_C"))
    (bind _output_get (Variables|Default|SetactualWidget _returnvalue))
    (UserInterface|Viewport|AddtoViewport _output_get 0)))

(event EventPossess
  (params (PossessedPawn :type Pawn%20Object%20Reference))
  (CallFunction|EventPossess))

(fn ConstructionScript)