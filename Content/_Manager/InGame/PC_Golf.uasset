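; Player controller for the golf game that prepares each player for match start and handles input locking.
; On possession it binds Start to the GS_Golf game-start event, disables pawn input, then after a short delay creates the in-game HUD widget.
; It then sets the RepNotify flag IsReady, whose OnRep asks GS_Golf to check player readiness.
; Start re-enables pawn input with the mouse cursor hidden.
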(event Custom|SetEnableInput
  (params (disable :type Boolean) (showMouse :type Boolean))
  (bind _self self)
  (bind _self_2 self)
  (bind _returnvalue (Pawn|GetControlledPawn _self))
  ;[0 0 0] Enable input
  (Variables|Default|SetbShowMouseCursor showMouse)
  (Utilities|IsValid _returnvalue
    (:Is%20Valid
      (if disable
        (Input|DisableInput _returnvalue _self_2)
        (else
          (Input|EnableInput _returnvalue _self_2))))))

(event Custom|Process%20Local
  ;[0 0 0] Initialize player
  (bind _returnvalue (UserInterface|CreateWidget "/Game/UI/InGame/WBP_InGame.WBP_InGame_C"))
  (bind _output_get (Variables|Default|SetactualWidget _returnvalue))
  (UserInterface|Viewport|AddtoViewport _output_get 0)
  (CallFunction|SetNotify))

(event Custom|SetNotify
  ;[0 0 0] Initialize player
  (Variables|Default|SetisReady true))

(event Custom|Start
  ;[0 0 0] Initialize player
  (CallFunction|SetEnableInput false false))

(event EventPossess
  (params (PossessedPawn :type Pawn%20Object%20Reference))
  ;[0 0 0] Initialize player
  (EventDispatchers|BindEventtoGameStart (.AsGS%20Golf (Utilities|Casting|CastToGS_Golf (Game|GetGameState))) (delegate Custom|Start))
  (CallFunction|SetEnableInput true false)
  (Utilities|FlowControl|Delay 1.0)
  (CallFunction|ProcessLocal))

(fn ConstructionScript)

(fn OnRepIsReady
  (Default|CheckPlayersReady (.AsGS%20Golf (Utilities|Casting|CastToGS_Golf (Game|GetGameState)))))