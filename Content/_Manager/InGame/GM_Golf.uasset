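; GM_Golf is the in-game golf game mode that spawns and possesses a BP_GolfPlayer for each player who logs in.
; It caches all PlayerStarts on first need and picks one by a running player index, falling back to a random start.
; Spawning keeps only the start's location and yaw and ignores collision.
; Each login then triggers LoadGame on GI_Golf, and logout decrements the index.
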(event EventPostLogin
  (params (NewPlayer :type Player%20Controller%20Object%20Reference))
  (bind _startref (Variables|Default|GetstartRef))
  (bind _playerindex (Variables|Default|GetplayerIndex))
  (bind _outitem (Utilities|Array|Random _startref))
  (bind _output (Utilities|Array|Get(acopy) _startref _playerindex))
  (bind _returnvalue (Utilities|IsValid _output))
  (bind _returnvalue_2 (select _returnvalue _output _outitem))
  (bind _returnvalue_3 (Transformation|GetActorTransform _returnvalue_2))
  ;[0 0 0] Player Log In
  (if (Utilities|Array|IsNotEmpty (Variables|Default|GetstartRef))
    _
    (else
      (|findPlayerStarts_2)))
  (bind _returnvalue_4 (Game|SpawnActorfromClass "/Game/Character/BP_GolfPlayer.BP_GolfPlayer_C" (Math|Transform|MakeTransform (.location _returnvalue_3) (Math|Rotator|MakeRotator 0.0 0.0 (.yaw (.rotation _returnvalue_3))) "1.000000,1.000000,1.000000") "AlwaysSpawn" "MultiplyWithRoot" 0 0))
  (Pawn|Possess NewPlayer _returnvalue_4)
  (Math|Integer|IncrementInt (Variables|Default|GetplayerIndex)
    (:%20%20
      (Default|LoadGame (.AsGI%20Golf (Utilities|Casting|CastToGI_Golf (Game|GetGameInstance)))))))

(event EventOnLogout
  (params (ExitingController :type Controller%20Object%20Reference))
  ;[0 0 0] player Log Out
  (Math|Integer|DecrementInt (Variables|Default|GetplayerIndex)))

(fn ConstructionScript)