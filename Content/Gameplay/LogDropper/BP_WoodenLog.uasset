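; BP_WoodenLog is a log dropper that repeatedly launches BP_Log actors in the golf game.
; It binds to the GS_Golf game-start event, then runs a looping spawn timer on the server only.
; Each tick of that timer spawns a log at the Arrow's transform, passes it a destroy delay, and pushes its capsule along the arrow's forward vector with a velocity-change impulse.
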(event Custom|Start
  (Networking|SwitchHasAuthority
    (:Authority
      (Utilities|Time|SetTimerbyEvent (delegate Custom|SpawnLog) (Variables|Default|GetspawnDelay) true))))

(event Custom|SpawnLog
  (bind _returnvalue (Game|SpawnActorfromClass "/Game/Gameplay/LogDropper/BP_Log.BP_Log_C" (Transformation|GetWorldTransform (Variables|Default|GetArrow)) "AlwaysSpawn" "MultiplyWithRoot" 0 (Variables|Default|GetdestroyDelay) 0))
  (Physics|AddImpulse (Variables|/Game/Gameplay/LogDropper/BP_Log.BP_Log_C|GetCapsule _returnvalue) (* (Math|Vector|GetForwardVector (Variables|Default|GetArrow)) 2.5e+02) "None" true))

(event EventBeginPlay
  (EventDispatchers|BindEventtoGameStart (.AsGS%20Golf (Utilities|Casting|CastToGS_Golf (Game|GetGameState))) (delegate Custom|Start)))

(fn ConstructionScript)