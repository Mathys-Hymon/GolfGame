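; BP_Hole is the golf hole actor that detects when a player finishes.
; A box overlap by a BP_GolfPlayer calls FinishedMessage on that player's PlayerState.
; The construction script picks the open, round or square hole mesh from the Open and Rounded flags, with Open taking priority.
; On BeginPlay, the BounceEffect timeline animates the flag's vertical scale for a bounce.
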(event OnComponentBeginOverlap(Box)
  (params (OverlappedComponent :type Primitive%20Component%20Object%20Reference) (OtherActor :type Actor%20Object%20Reference) (OtherComp :type Primitive%20Component%20Object%20Reference) (OtherBodyIndex :type Integer) (bFromSweep :type Boolean) (SweepResult :type Hit%20Result%20Structure%20%28by%20ref%29))
  (bind _asbp_golf_player (Utilities|Casting|CastToBP_GolfPlayer OtherActor))
  (Class|BPIPlayerInfo|Finished(Message) (Variables|/Script/Engine.Pawn|GetPlayerState _asbp_golf_player)))

(event EventBeginPlay
  ;[0 0 0] Bounce flag
  (bind _lerp (Timeline|bounceEffect Play)
    (:Update
      (Transformation|SetWorldScale3D (Variables|Default|Getflag) (Math|Vector|MakeVector 1.0 1.0 _lerp)))))

(fn ConstructionScript
  (if (Variables|Default|Getopen)
    (Components|StaticMesh|SetStaticMesh (Variables|Default|GetStaticMesh) "/Game/Art/Mesh/hole-open_hole-open.hole-open_hole-open")
    (elif (Variables|Default|Getrounded)
      (Components|StaticMesh|SetStaticMesh (Variables|Default|GetStaticMesh) "/Game/Art/Mesh/hole-round_hole-round.hole-round_hole-round")
      (else
        (Components|StaticMesh|SetStaticMesh (Variables|Default|GetStaticMesh) "/Game/Art/Mesh/hole-square_hole-square.hole-square_hole-square")))))