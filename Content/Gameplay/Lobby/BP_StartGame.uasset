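; BP_StartGame is a lobby start-game zone that tracks how many overlaps are inside its Sphere as a ready count.
; Overlap begin and end raise or lower PlayerReady without filtering by actor type, then pass the count to CheckEveryoneReady on the GS_Lobby game state.
; On BeginPlay, a timeline drives the Flag's vertical world scale.
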(event OnComponentBeginOverlap(Sphere)
  (params (OverlappedComponent :type Primitive%20Component%20Object%20Reference) (OtherActor :type Actor%20Object%20Reference) (OtherComp :type Primitive%20Component%20Object%20Reference) (OtherBodyIndex :type Integer) (bFromSweep :type Boolean) (SweepResult :type Hit%20Result%20Structure%20%28by%20ref%29))
  (Math|Integer|IncrementInt (Variables|Default|GetplayerReady)
    (:%20%20
      (Default|CheckEveryoneReady (.AsGS%20Lobby (Utilities|Casting|CastToGS_Lobby (Game|GetGameState))) (Variables|Default|GetplayerReady)))))

(event OnComponentEndOverlap(Sphere)
  (params (OverlappedComponent :type Primitive%20Component%20Object%20Reference) (OtherActor :type Actor%20Object%20Reference) (OtherComp :type Primitive%20Component%20Object%20Reference) (OtherBodyIndex :type Integer))
  (Math|Integer|DecrementInt (Variables|Default|GetplayerReady)
    (:%20%20
      (Default|CheckEveryoneReady (.AsGS%20Lobby (Utilities|Casting|CastToGS_Lobby (Game|GetGameState))) (Variables|Default|GetplayerReady)))))

(event EventBeginPlay
  (bind _lerp (Timeline|Timeline Play)
    (:Update
      (Transformation|SetWorldScale3D (Variables|Default|Getflag) (Math|Vector|MakeVector 1.0 1.0 _lerp)))))

(fn ConstructionScript)