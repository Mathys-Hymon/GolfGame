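; BP_SkinChanger is a lobby floor button that cycles a player's skin or hat when stepped on, chosen by a SkinButton flag that also sets its label.
; Overlap plays a timeline that lowers the button mesh, and end overlap reverses it.
; If still pressed when the timeline finishes, the server takes the first overlapping BP_LobbyPlayer and calls increment skin or hat on its PS_Lobby player state.
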(event OnComponentBeginOverlap(Box)
  (params (OverlappedComponent :type Primitive%20Component%20Object%20Reference) (OtherActor :type Actor%20Object%20Reference) (OtherComp :type Primitive%20Component%20Object%20Reference) (OtherBodyIndex :type Integer) (bFromSweep :type Boolean) (SweepResult :type Hit%20Result%20Structure%20%28by%20ref%29))
  (bind _box (Variables|Default|GetBox))
  (bind _overlappingactors (Collision|GetOverlappingActors _box "/Game/Character/BP_LobbyPlayer.BP_LobbyPlayer_C" :!class /Script/Engine.PrimitiveComponent))
  (bind _output (Utilities|Array|Get(acopy) _overlappingactors))
  (bind _asbp_lobby_player (Utilities|Casting|CastToBP_LobbyPlayer _output))
  (bind _playerstate (Variables|/Script/Engine.Pawn|GetPlayerState _asbp_lobby_player))
  (bind _asps_lobby (Utilities|Casting|CastToPS_Lobby _playerstate))
  ;[0 0 0] Change Skin/hat when player walk on it
  (Variables|Default|Setpressed true)
  (bind _alpha (Timeline|setButton Play)
    (:Update
      (Transformation|SetRelativeLocation (Variables|Default|GetSM_Button) (Math|Vector|Lerp(Vector) "0, 0, 0" "0.000000,0.000000,-14.000000" _alpha) false true))
    (:Finished
      (if (Variables|Default|Getpressed)
        (Networking|SwitchHasAuthority
          (:Authority
            (if (Variables|Default|GetskinButton)
              (Default|SRVIncrementSkin _asps_lobby)
              (else
                (Default|SRVIncrementHat _asps_lobby)))))))))

(event OnComponentEndOverlap(Box)
  (params (OverlappedComponent :type Primitive%20Component%20Object%20Reference) (OtherActor :type Actor%20Object%20Reference) (OtherComp :type Primitive%20Component%20Object%20Reference) (OtherBodyIndex :type Integer))
  (bind _box (Variables|Default|GetBox))
  (bind _overlappingactors (Collision|GetOverlappingActors _box "/Game/Character/BP_LobbyPlayer.BP_LobbyPlayer_C" :!class /Script/Engine.PrimitiveComponent))
  (bind _output (Utilities|Array|Get(acopy) _overlappingactors))
  (bind _asbp_lobby_player (Utilities|Casting|CastToBP_LobbyPlayer _output))
  (bind _playerstate (Variables|/Script/Engine.Pawn|GetPlayerState _asbp_lobby_player))
  (bind _asps_lobby (Utilities|Casting|CastToPS_Lobby _playerstate))
  ;[0 0 0] Change Skin/hat when player walk on it
  (Variables|Default|Setpressed false)
  (bind _alpha (Timeline|setButton Reverse)
    (:Update
      (Transformation|SetRelativeLocation (Variables|Default|GetSM_Button) (Math|Vector|Lerp(Vector) "0, 0, 0" "0.000000,0.000000,-14.000000" _alpha) false true))
    (:Finished
      (if (Variables|Default|Getpressed)
        (Networking|SwitchHasAuthority
          (:Authority
            (if (Variables|Default|GetskinButton)
              (Default|SRVIncrementSkin _asps_lobby)
              (else
                (Default|SRVIncrementHat _asps_lobby)))))))))

(fn ConstructionScript
  (Rendering|Components|TextRender|SetText (Variables|Default|Gettext) (Utilities|String|SelectText "skin" "hat" (Variables|Default|GetskinButton))))