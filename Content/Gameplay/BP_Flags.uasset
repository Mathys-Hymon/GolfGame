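; Flag actor that shows a selectable flag mesh and animates it with a gentle rotation.
; The construction script applies the chosen mesh to the Flag component.
; On BeginPlay, a random delay of up to one second staggers a timeline that adds small yaw rotations each update.
; An Odd toggle flips the rotation direction.
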(event EventBeginPlay
  (Utilities|FlowControl|Delay (Math|Random|RandomFloatinRange 0.0 1.0))
  (bind _lerp (Timeline|Timeline Play)
    (:Update
      (Transformation|AddWorldRotation (Variables|Default|Getflag) (Math|Rotator|MakeRotator 0.0 0.0 (Math|Float|SelectFloat (/ _lerp 5.0) (* (/ _lerp 5.0) -1.0) (Variables|Default|Getodd))) false false))))

(fn ConstructionScript
  (Components|StaticMesh|SetStaticMesh (Variables|Default|Getflag) (Variables|Default|GetflagType)))