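; BP_LobbyPlayer is the lobby player pawn: a physics ball with a dynamic material, a swappable hat and a name widget.
; Enhanced Input drives camera look, control-yaw-relative force and impulse jumps, with movement and jumps routed through SRV-to-MC event pairs for networking.
; Hits on the ground physical material re-enable jumping.
; The detached name pivot follows the ball each tick while the widget turns to face the local camera.
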(event OnComponentHit(Sphere)
  (params (HitComponent :type Primitive%20Component%20Object%20Reference) (OtherActor :type Actor%20Object%20Reference) (OtherComp :type Primitive%20Component%20Object%20Reference) (NormalImpulse :type Vector :default "0, 0, 0") (Hit :type Hit%20Result%20Structure%20%28by%20ref%29))
  ;[0 0 0] Detect Ground
  (if (and (not (Variables|Default|GetisGrounded)) (== (.PhysMat (Collision|BreakHitResult Hit)) "/Game/Art/Materials/Physics/PM_Ground.PM_Ground"))
    (Variables|Default|SetisGrounded true)))

(event Custom|possess
  (params (newController :type Controller%20Object%20Reference))
  ;[0 0 0] Begin Play
  (bind _aspc_lobby (Utilities|Casting|CastToPC_Lobby newController))
  (Utilities|IsValid (PlayerController|LocalPlayerSubsystems|GetEnhancedInputLocalPlayerSubsystem _aspc_lobby)
    (:Is%20Valid
      (Input|AddMappingContext (PlayerController|LocalPlayerSubsystems|GetEnhancedInputLocalPlayerSubsystem _aspc_lobby) "/Game/Gameplay/Inputs/Lobby/IMC_Lobby.IMC_Lobby" 0 "(bIgnoreAllPressedKeysUntilRelease=True,bForceImmediately=False,bNotifyUserSettings=False)"))))

(event Custom|JumpSRV
  ;[0 0 0] Jump Event
  (CallFunction|JumpMC))

(event Custom|JumpMC
  ;[0 0 0] Jump Event
  (Physics|AddImpulse (Variables|Default|GetSphere) "0.000000,0.000000,500.000000" "None" true)
  (Variables|Default|SetisGrounded false))

(event Custom|MoveSRV
  (params (velocity :type Vector))
  ;[0 0 0] Movement
  (CallFunction|MoveMC velocity))

(event Custom|MoveMC
  (params (Force :type Vector))
  ;[0 0 0] Movement
  (Physics|AddForce (Variables|Default|GetSphere) Force "None" true))

(event Input|EnhancedActionEvents|EnhancedInputActionIA_Look
  (params (ActionValue :type Vector%202D%20Structure) (ElapsedSeconds :type Float%20%28double-precision%29) (TriggeredSeconds :type Float%20%28double-precision%29) (InputAction :type Input%20Action%20Object%20Reference :default "/Game/Gameplay/Inputs/InGame/Actions/IA_Look.IA_Look"))
  ;[0 0 0] CameraRotation
  (Pawn|Input|AddControllerYawInput (.x ActionValue))
  (Pawn|Input|AddControllerPitchInput (* (.y ActionValue) -1.0)))

(event Input|EnhancedActionEvents|EnhancedInputActionIA_Move
  (params (ActionValue :type Vector%202D%20Structure) (ElapsedSeconds :type Float%20%28double-precision%29) (TriggeredSeconds :type Float%20%28double-precision%29) (InputAction :type Input%20Action%20Object%20Reference :default "/Game/Gameplay/Inputs/Lobby/Actions/IA_Move.IA_Move"))
  (bind _returnvalue (Pawn|GetController))
  (bind _returnvalue_2 (* ActionValue 5e+02))
  (bind _returnvalue_3 (Pawn|GetControlRotation _returnvalue :!class /Script/Engine.Controller))
  (bind _returnvalue_4 (Math|Rotator|MakeRotator 0.0 0.0 (.yaw _returnvalue_3)))
  ;[0 0 0] Movement
  (CallFunction|MoveSRV (+ (* (.x _returnvalue_2) (Math|Vector|GetForwardVector _returnvalue_4)) (* (.y _returnvalue_2) (Math|Vector|GetRightVector _returnvalue_4) -1.0))))

(event Input|EnhancedActionEvents|EnhancedInputActionIA_Jump
  (params (ActionValue :type Boolean) (ElapsedSeconds :type Float%20%28double-precision%29) (TriggeredSeconds :type Float%20%28double-precision%29) (InputAction :type Input%20Action%20Object%20Reference :default "/Game/Gameplay/Inputs/Lobby/Actions/IA_Jump.IA_Jump"))
  ;[0 0 0] Jump Event
  (:Started
    (if (Variables|Default|GetisGrounded)
      (Networking|SwitchHasAuthority
        (:Authority
          (CallFunction|JumpMC))
        (:Remote
          (CallFunction|JumpSRV))))))

(event EventSetHat
  (params (newMesh :type Static%20Mesh%20Object%20Reference))
  (Components|StaticMesh|SetStaticMesh (Variables|Default|Gethat) newMesh))

(event EventSetName
  (params (name :type String) (color :type Vector :default "0, 0, 0"))
  ;[0 0 0] Player Set Name
  (Class|BPIPlayer|SetName(Message) (UserInterface|GetWidget (Variables|Default|GetuserInfo)) name color))

(event EventPossessed
  (params (NewController :type Controller%20Object%20Reference))
  ;[0 0 0] Begin Play
  (CallFunction|Possess NewController))

(event EventTick
  (params (DeltaSeconds :type Float%20%28single-precision%29))
  (bind _userinfo (Variables|Default|GetuserInfo))
  ;[0 0 0] Rotate Name
  (Transformation|SetWorldRotation _userinfo (Math|Rotator|FindLookatRotation (Transformation|GetWorldLocation _userinfo) (Transformation|GetWorldLocation (Variables|/Script/Engine.PlayerCameraManager|GetTransformComponent (Game|GetPlayerCameraManager 0)))) false false)
  (Transformation|SetWorldLocation (Variables|Default|GetnamePivot) (Transformation|GetActorLocation) false false))

(event EventBeginPlay
  (bind _namepivot (Variables|Default|GetnamePivot))
  ;[0 0 0] Begin Play
  (bind _returnvalue (Rendering|Material|CreateDynamicMaterialInstance "/Game/Art/Materials/MI_Ball.MI_Ball" "None" "None" :!class /Script/Engine.KismetMaterialLibrary))
  (bind _output_get (Variables|Default|SetdynamicMat _returnvalue))
  (Rendering|Material|SetMaterial (Variables|Default|GetSM_Ball) 0 _output_get)
  (Utilities|IsValid (Components|GetOwner _namepivot)
    (:Is%20Valid
      (Transformation|DetachFromComponent _namepivot "KeepWorld" "KeepWorld" "KeepWorld" true)
      (Transformation|SetWorldRotation _namepivot "0, 0, 0" false false))))

(fn ConstructionScript)

(fn GetBallMaterial
  (return (Variables|Default|GetdynamicMat)))