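; Player-controlled golf ball pawn for multiplayer, with name display, hat, dynamic material and impact sounds.
; While the slow ball is charged, vertical look input moves the club, and crossing the ball applies a velocity-scaled impulse through AddBallForceMC.
; Resting saves the respawn point and shows a local aim preview; respawn and spectate propagate through MC events.
; Tick billboards the name, turns the hat and adjusts linear damping by speed and surface contact.
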(event OnComponentHit(Sphere)
  (params (HitComponent :type Primitive%20Component%20Object%20Reference) (OtherActor :type Actor%20Object%20Reference) (OtherComp :type Primitive%20Component%20Object%20Reference) (NormalImpulse :type Vector :default "0, 0, 0") (Hit :type Hit%20Result%20Structure%20%28by%20ref%29))
  (bind _returnvalue (Math|Vector|VectorLength NormalImpulse))
  ;[0 0 0] Play SFX
  (if (> _returnvalue 1.5e+03)
    (CallFunction|PlayHitSound _returnvalue)))

(event Custom|possess
  (params (newController :type Controller%20Object%20Reference))
  ;[0 0 0] Begin Play
  (bind _aspc_golf (Utilities|Casting|CastToPC_Golf newController))
  (Utilities|IsValid (PlayerController|LocalPlayerSubsystems|GetEnhancedInputLocalPlayerSubsystem _aspc_golf)
    (:Is%20Valid
      (Input|AddMappingContext (PlayerController|LocalPlayerSubsystems|GetEnhancedInputLocalPlayerSubsystem _aspc_golf) "/Game/Gameplay/Inputs/InGame/IMC_Golf.IMC_Golf" 0 "(bIgnoreAllPressedKeysUntilRelease=True,bForceImmediately=False,bNotifyUserSettings=False)"))))

(event Custom|AddBallForceMC
  (params (Impulse :type Vector))
  ;[0 0 0] Add Force
  (Physics|AddImpulse (Variables|Default|GetSphere) Impulse "None" true)
  (Variables|ClubHit|SethitVelocity 0.0)
  (Variables|ClubHit|SethitOffset 0.0))

(event Custom|SpectateLocal
  ;[0 0 0] Spectate Mode
  (Transformation|DetachFromComponent (Variables|Default|GetSpringArm) "KeepWorld" "KeepWorld" "KeepWorld" true)
  (CallFunction|Respawn))

(event Custom|SpectateModeMC
  ;[0 0 0] Spectate Mode
  (Variables|Default|SetrespawnLoc "0.000000,0.000000,-500.000000")
  (CallFunction|SpectateLocal)
  (Rendering|SetVisibility (Variables|Default|GetuserInfo) false false))

(event Custom|AddBallForce
  (params (Impulse :type Vector))
  ;[0 0 0] Add Force
  (CallFunction|AddBallForceMC Impulse))

(event Custom|PlayHitSound
  (params (hitVolume :type Float%20%28double-precision%29))
  ;[0 0 0] Play SFX
  (Audio|SpawnSoundatLocation "/Game/Art/SFX/ballHit.ballHit" (Transformation|GetActorLocation) "0, 0, 0" (Math|Float|Clamp(Float) (/ hitVolume 1.2e+04) 0.0 0.8) (Math|Random|RandomFloatinRange 0.9 1.1) 0.0 "/Game/Art/SFX/NewSoundAttenuation.NewSoundAttenuation" 0))

(event Custom|ShowClub
  (params (show :type Boolean))
  (bind _returnvalue (Pawn|GetController))
  (bind _returnvalue_2 (Pawn|GetControlRotation _returnvalue :!class /Script/Engine.Controller))
  (bind _returnvalue_3 (Math|Rotator|MakeRotator 0.0 0.0 (.yaw _returnvalue_2)))
  ;[0 0 0] Show Club
  (Rendering|SetVisibility (Variables|Default|Getclub) show true)
  (Transformation|SetWorldLocationAndRotation (Variables|Default|Getclub) (+ (Transformation|GetActorLocation) (* (Math|Vector|GetForwardVector _returnvalue_3) (Variables|ClubHit|GethitOffset) -1.0)) _returnvalue_3 false false))

(event Custom|ShowPreviewLocal
  (params (show :type Boolean))
  ;[0 0 0] Rotate Preview Direction
  (if (Pawn|IsLocallyControlled)
    (Rendering|SetVisibility (Variables|Default|GetpreviewPivot) show true)
    (Utilities|IsValid (Pawn|GetController)
      (:Is%20Valid
        (if show
          (bind _returnvalue (Utilities|Time|SetTimerbyEvent (delegate Custom|UpdateRotationPlane) 0.001 true true))
          (elif (Utilities|Time|IsValidTimerHandle _returnvalue)
            (Utilities|Time|PauseTimerbyHandle _returnvalue)))))))

(event Custom|UpdateRotationPlane
  ;[0 0 0] Rotate Preview Direction
  (Transformation|SetWorldRotation (Variables|Default|GetpreviewPivot) (Math|Conversions|RotationFromXVector (* (Math|Vector|GetRightVector (Math|Rotator|MakeRotator 0.0 0.0 (.yaw (Pawn|GetControlRotation (Pawn|GetController) :!class /Script/Engine.Controller)))) -1.0)) false false))

(event Custom|RespawnSRV
  ;[0 0 0] Respawn
  (CallFunction|RespawnMC))

(event Custom|RespawnMC
  (bind _respawnloc (Variables|Default|GetrespawnLoc))
  (bind _sphere (Variables|Default|GetSphere))
  ;[0 0 0] Respawn
  (if (Utilities|Operators|NotEqual(!=) :A _respawnloc)
    (Transformation|SetActorLocation _respawnloc false true)
    (Physics|SetSimulatePhysics _sphere false)
    (Utilities|FlowControl|DelayUntilNextTick)
    (Physics|SetSimulatePhysics _sphere true)))

(event Custom|SpectateMode
  ;[0 0 0] Spectate Mode
  (CallFunction|SpectateModeMC))

(event Input|EnhancedActionEvents|EnhancedInputActionIA_Look
  (params (ActionValue :type Vector%202D%20Structure) (ElapsedSeconds :type Float%20%28double-precision%29) (TriggeredSeconds :type Float%20%28double-precision%29) (InputAction :type Input%20Action%20Object%20Reference :default "/Game/Gameplay/Inputs/InGame/Actions/IA_Look.IA_Look"))
  (bind _returnvalue (* (.y ActionValue) 3.0))
  ;[0 0 0] Look Rotation
  (if (Variables|Default|GetunlockCamera)
    (if (Variables|ClubHit|GetchargeAttack)
      (Variables|ClubHit|SethitVelocity _returnvalue)
      (bind _output_get (Variables|ClubHit|SethitOffset (- (Variables|ClubHit|GethitOffset) _returnvalue)))
      (if (not (> _output_get 0.0))
        (Variables|ClubHit|SetchargeAttack false)
        (Utilities|FlowControl|DoOnce false :!label _label
          (:Completed
            (Audio|PlaySound2D "/Game/Art/SFX/putterHit.putterHit" 1.0 1.0 0.0 0 0)
            (CallFunction|AddBallForce (* (Math|Vector|GetForwardVector (Math|Rotator|MakeRotator 0.0 0.0 (.yaw (Pawn|GetControlRotation (Pawn|GetController) :!class /Script/Engine.Controller)))) (Variables|ClubHit|GethitVelocity) 1.5e+02))
            (Rendering|SetVisibility (Variables|Default|Getclub) false true)
            (Class|BPIPlayerInfo|IncreaseHit(Message) (Variables|/Script/Engine.Controller|GetPlayerState (Pawn|GetController))))))
      (else
        (Variables|ClubHit|SethitVelocity 0.0 :!label _label_2)
        (Variables|ClubHit|SethitOffset 15.0)
        (goto _label Reset)))
    (else
      (Pawn|Input|AddControllerYawInput (.x ActionValue))
      (Pawn|Input|AddControllerPitchInput (* (.y ActionValue) -1.0))
      (goto _label_2))))

(event Input|EnhancedActionEvents|EnhancedInputActionIA_Charge
  (params (ActionValue :type Boolean) (ElapsedSeconds :type Float%20%28double-precision%29) (TriggeredSeconds :type Float%20%28double-precision%29) (InputAction :type Input%20Action%20Object%20Reference :default "/Game/Gameplay/Inputs/InGame/Actions/IA_Charge.IA_Charge"))
  ;[0 0 0] Charge Click
  (:Triggered
    (if (< (Math|Vector|VectorLength (Transformation|GetVelocity)) 35.0) :!label _label
      (bind _output_get (Variables|ClubHit|SetchargeAttack ActionValue))
      (CallFunction|ShowClub _output_get)
      (Variables|Default|SetunlockCamera _output_get)
      (else
        (if ActionValue
          _
          (else
            (Variables|Default|SetunlockCamera false)))
        (CallFunction|ShowClub false))))
  (:Canceled
    (goto _label))
  (:Completed
    (goto _label)))

(event Input|EnhancedActionEvents|EnhancedInputActionIA_Respawn
  (params (ActionValue :type Boolean) (ElapsedSeconds :type Float%20%28double-precision%29) (TriggeredSeconds :type Float%20%28double-precision%29) (InputAction :type Input%20Action%20Object%20Reference :default "/Game/Gameplay/Inputs/InGame/Actions/IA_Respawn.IA_Respawn"))
  ;[0 0 0] Respawn
  (:Started
    (CallFunction|Respawn)))

(event EventRespawn
  ;[0 0 0] Respawn
  (Networking|SwitchHasAuthority
    (:Authority
      (CallFunction|RespawnMC))
    (:Remote
      (CallFunction|RespawnSRV))))

(event EventPossessed
  (params (NewController :type Controller%20Object%20Reference))
  ;[0 0 0] Begin Play
  (CallFunction|Possess NewController))

(event EventTick
  (params (DeltaSeconds :type Float%20%28single-precision%29))
  ;[0.05208 0 0] Tick
  (|UpdateName
    (:execute
      (if (< (Math|Vector|VectorLength (Transformation|GetVelocity)) 35.0)
        (Utilities|FlowControl|DoOnce false :!label _label
          (:Completed
            (Utilities|FlowControl|Sequence
              (:then_0
                (CallFunction|ShowPreviewLocal true)
                (Variables|Default|SetrespawnLoc (Transformation|GetActorLocation)))
              (:then_1
                (goto _label_2 Reset)))))
        (else
          (Utilities|FlowControl|DoOnce false :!label _label_2
            (:Completed
              (Utilities|FlowControl|Sequence
                (:then_0
                  (goto _label Reset))
                (:then_1
                  (CallFunction|ShowPreviewLocal false))))))))))

(event EventBeginPlay
  (bind _namepivot (Variables|Default|GetnamePivot))
  ;[0 0 0] Begin Play
  (bind _returnvalue (Rendering|Material|CreateDynamicMaterialInstance "/Game/Art/Materials/MI_Ball.MI_Ball" "None" "None" :!class /Script/Engine.KismetMaterialLibrary))
  (bind _output_get (Variables|Default|SetdynamicMat _returnvalue))
  (Rendering|Material|SetMaterial (Variables|Default|GetSM_Ball) 0 _output_get)
  (Utilities|IsValid (Components|GetOwner _namepivot)
    (:Is%20Valid
      (Transformation|DetachFromComponent _namepivot "KeepWorld" "KeepWorld" "KeepWorld" true)
      (Transformation|SetWorldRotation _namepivot "0, 0, 0" false false))))

(event EventSetHat
  (params (newMesh :type Static%20Mesh%20Object%20Reference))
  ;[0 0 0] Begin Play
  (Components|StaticMesh|SetStaticMesh (Variables|Default|Gethat) newMesh))

(event EventSetName
  (params (name :type String) (color :type Vector :default "0, 0, 0"))
  ;[0 0 0] Player Set Name
  (Class|BPIPlayer|SetName(Message) (UserInterface|GetWidget (Variables|Default|GetuserInfo)) name color))

(fn ConstructionScript)

(fn GetBallMaterial
  (return (Variables|Default|GetdynamicMat)))